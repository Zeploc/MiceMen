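; Game mode Blueprint for a turn-based team game, showing debug state and the end screen.
; Every tick it prints the current player and each TeamPoints score to screen, labeling teams by loop index rather than map key.
; When a team wins, it creates the MM_UI_EndScreen widget, sets the winning team and adds it to the viewport.
; The turn-switch event is an empty stub.
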(event `self.ReceiveBeginPlay`)

(event `self.ReceiveTick`
  (params (DeltaSeconds :type "Float (single-precision)"))
  (`KismetSystemLibrary.PrintString` (`KismetStringLibrary.Concat_StrStr` "Current Player: " (`KismetSystemLibrary.GetDisplayName` (`self.CurrentPlayer`))) true false (struct :`R` 0.982312 :`G` 0.613319 :`B` 1.0 :`A` 1.0) DeltaSeconds)
  (bind _keys (`BlueprintMapLibrary.Map_Keys` (`self.TeamPoints`)))
  (for (_array_element _array_index) _keys
    (`KismetSystemLibrary.PrintString` (`KismetStringLibrary.Concat_StrStr` "Team " (`KismetStringLibrary.Conv_IntToString` _array_index) ": " (`KismetStringLibrary.Conv_IntToString` (`BlueprintMapLibrary.Map_Find` (`self.TeamPoints`) _array_element))) true false (struct :`R` 0.263283 :`G` 0.305833 :`B` 1.0 :`A` 1.0) DeltaSeconds)))

(event `self.BI_OnSwitchTurns`
  (params (_Player :type "MM_PlayerController Object Reference")))

(fn `BI_OnTeamWon`
  (params (_iTeam :type Integer))
  (bind _returnvalue (`|CreateWidget` "/Game/UI/MM_UI_EndScreen.MM_UI_EndScreen_C"))
  (`/Game/UI/MM_UI_EndScreen.SetWinningTeam` _returnvalue (`local._iTeam`))
  (`UserWidget.AddToViewport` _returnvalue 0))

(fn `UserConstructionScript`)