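; Column control Blueprint that shows a team-coloured highlight when it is flagged as grabbable.
; On BeginPlay it sizes the ColumnHighlight to the GrabbableBox bounds, hides it and creates a dynamic material instance for it.
; BI_DisplayGrabbable toggles the highlight's visibility and, when grabbable, sets its Colour parameter from the MM singleton's TeamColours map.
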(event `self.ReceiveBeginPlay`
  (`parent.ReceiveBeginPlay`)
  (`SceneComponent.SetRelativeScale3D` (`self.ColumnHighlight`) (/ (`.BoxExtent` (`KismetSystemLibrary.GetComponentBounds` (`self.GrabbableBox`))) 50.0))
  (`SceneComponent.SetVisibility` (`self.ColumnHighlight`) false false)
  (bind _returnvalue (`PrimitiveComponent.CreateDynamicMaterialInstance` (`self.ColumnHighlight`) 0 null "None"))
  (set `self.HighlightDMI` _returnvalue))

(fn `BI_DisplayGrabbable`
  (params (_bGrabbable :type Boolean) (_Team :type Integer))
  (bind _returnvalue (`MM_FunctionLibrary.GetMMSingleton`))
  (bind (_value _returnvalue_2) (`BlueprintMapLibrary.Map_Find` (`MM_Singleton.TeamColours` _returnvalue) (`local._Team`)))
  (`SceneComponent.SetVisibility` (`self.ColumnHighlight`) (`local._bGrabbable`) false)
  (if (`local._bGrabbable`)
    (`/Engine/EditorBlueprintResources/StandardMacros.IsValid` _returnvalue
      (:`Is Valid`
        (if _returnvalue_2
          (bind _highlightdmi (`self.HighlightDMI`)
            (:`then`
              (`MaterialInstanceDynamic.SetVectorParameterValue` _highlightdmi "Colour" _value))
            (:`else`)))))))

(fn `UserConstructionScript`)