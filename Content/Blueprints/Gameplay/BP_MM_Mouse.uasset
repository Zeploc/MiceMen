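; BP_MM_Mouse is a team-coloured mouse actor that hops along a supplied path of points.
; On BeginPlay it tints its sphere through a dynamic material instance, choosing one of two colours by team.
; The BIMoveAlongPath event stores the path, then a timeline lerps the actor between the first two points with an added height offset.
; When each hop finishes, it removes the first point and recurses until no next point remains.
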(event `self.ReceiveBeginPlay`
  (bind _returnvalue (`PrimitiveComponent.CreateDynamicMaterialInstance` (`self.Sphere`) 0 null "None"))
  (`MaterialInstanceDynamic.SetVectorParameterValue` _returnvalue "Colour" (select `int` (`self.iTeam`) :`0` (struct :`R` 0.07451 :`G` 0.384314 :`B` 0.560784 :`A` 1.0) :`1` (struct :`R` 0.698039 :`G` 0.047263 :`B` 0.072855 :`A` 1.0) :!type "LinearColor Structure")))

(event `self.BI_MoveAlongPath`
  (params (_Path :type "Array of Vector Structure (by ref)"))
  (set `self.CurrentPath` _Path)
  (`self.MoveToNextPoint` (`self.CurrentPath`)))

(event `MoveToNextPoint`
  (params (NextPoints :type "Array of Vector Structure"))
  (if (`KismetArrayLibrary.Array_IsValidIndex` NextPoints 1)
    (bind (_direction _height _percentage) (`Timeline|MoveToPoint` :!via `PlayFromStart`)
      (:`Update`
        (bind (_returnvalue_x _returnvalue_y _returnvalue_z) (`KismetMathLibrary.BreakVector` (`KismetMathLibrary.VLerp` (`|GetArrayItem` NextPoints) (`|GetArrayItem` NextPoints 1) _percentage)))
        (`self.K2_SetActorLocation` (`KismetMathLibrary.MakeVector` _returnvalue_x _returnvalue_y (+ _returnvalue_z (* _height 25.0)))))
      (:`Finished`
        (`KismetArrayLibrary.Array_Remove` (`self.CurrentPath`))
        (`self.MoveToNextPoint` (`self.CurrentPath`))))))

(fn `UserConstructionScript`)