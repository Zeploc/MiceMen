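; Game mode Blueprint that manages the UI of a turn-based team game.
; When the game is ready it creates start, HUD and end screen widgets, then toggles their visibility as games begin and end.
; Team-win and turn-switch callbacks pass the winner, reason or active player to the end screen and HUD.
; Tick prints the current player controller and each team's points on screen as debug output.
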(event `self.ReceiveBeginPlay`
  (`parent.ReceiveBeginPlay`))

(event `self.ReceiveTick`
  (params (DeltaSeconds :type "Float (single-precision)"))
  (`KismetSystemLibrary.PrintString` (`KismetStringLibrary.Concat_StrStr` "Current Player: " (`KismetSystemLibrary.GetDisplayName` (`self.CurrentPlayerController`))) true false (struct :`R` 0.982312 :`G` 0.613319 :`B` 1.0 :`A` 1.0) DeltaSeconds)
  (bind _keys (`BlueprintMapLibrary.Map_Keys` (`self.TeamPoints`)))
  (for (_array_element _array_index) _keys
    (`KismetSystemLibrary.PrintString` (`KismetStringLibrary.Concat_StrStr` "Team " (`KismetStringLibrary.Conv_IntToString` _array_index) ": " (`KismetStringLibrary.Conv_IntToString` (`BlueprintMapLibrary.Map_Find` (`self.TeamPoints`) _array_element))) true false (struct :`R` 0.263283 :`G` 0.305833 :`B` 1.0 :`A` 1.0) DeltaSeconds)))

(fn `BI_OnGameBegun`
  (`|ExecutionSequence`
    (:`then_0`
      ;[1 1 1] Display HUD
      (bind _uihud (`self.UIHUD`)
        (:`then`
          (`Widget.SetVisibility` _uihud "SelfHitTestInvisible")
          (`/Game/UI/MM_UI_HUD.NewGameStarted` (`self.UIHUD`)))
        (:`else`)))
    (:`then_1`
      ;[1 1 1] Hide Other screens
      (bind _uistartscreen (`self.UIStartScreen`)
        (:`then`
          (`Widget.SetVisibility` _uistartscreen "Collapsed"))
        (:`else`)))
    (:`then_2`
      (bind _endscreen (`self.EndScreen`)
        (:`then`
          (`Widget.SetVisibility` _endscreen "Collapsed"))
        (:`else`)))))

(fn `BI_OnGameEnded`
  (`|ExecutionSequence`
    (:`then_0`
      ;[1 1 1] Display Menu Screen
      (bind _uistartscreen (`self.UIStartScreen`)
        (:`then`
          (`Widget.SetVisibility` _uistartscreen "SelfHitTestInvisible"))
        (:`else`)))
    (:`then_1`
      ;[1 1 1] Hide Other screens
      (bind _uihud (`self.UIHUD`)
        (:`then`
          (`Widget.SetVisibility` _uihud "Collapsed"))
        (:`else`)))
    (:`then_2`
      (bind _endscreen (`self.EndScreen`)
        (:`then`
          (`Widget.SetVisibility` _endscreen "Collapsed"))
        (:`else`)))))

(fn `BI_OnGameReady`
  (`self.CreateUIScreens`))

(fn `BI_OnSwitchTurns`
  (params (_Player :type "MM_PlayerController Object Reference"))
  (bind _uihud (`self.UIHUD`)
    (:`then`
      (`/Game/UI/MM_UI_HUD.SwitchPlayers` _uihud (`local._Player`)))
    (:`else`)))

(fn `BI_OnTeamWon`
  (params (_Team :type "ETeam Enum" :default "E_NONE") (_Reason :type String))
  (bind _endscreen (`self.EndScreen`)
    (:`then`
      (`/Game/UI/MM_UI_EndScreen.SetWinningTeam` _endscreen (`local._Team`) (`local._Reason`))
      (`Widget.SetVisibility` (`self.EndScreen`) "SelfHitTestInvisible"))
    (:`else`)))

(fn `CreateUIScreens`
  (`|ExecutionSequence`
    (:`then_0`
      (bind _returnvalue (`|CreateWidget` "/Game/UI/MM_UI_StartScreen.MM_UI_StartScreen_C" null self))
      (bind _output_get (set `self.UIStartScreen` _returnvalue))
      (`UserWidget.AddToViewport` _output_get 0))
    (:`then_1`
      (bind _returnvalue_2 (`|CreateWidget` "/Game/UI/MM_UI_HUD.MM_UI_HUD_C" null self))
      (bind _output_get_2 (set `self.UIHUD` _returnvalue_2))
      (`UserWidget.AddToViewport` _output_get_2 1)
      (`Widget.SetVisibility` (`self.UIHUD`) "Collapsed") ; Not initially visible
    )
    (:`then_2`
      (bind _returnvalue_3 (`|CreateWidget` "/Game/UI/MM_UI_EndScreen.MM_UI_EndScreen_C"))
      (bind _output_get_3 (set `self.EndScreen` _returnvalue_3))
      (`UserWidget.AddToViewport` _output_get_3 0)
      (`Widget.SetVisibility` (`self.EndScreen`) "Collapsed") ; Not initially visible
    )))

(fn `UserConstructionScript`)