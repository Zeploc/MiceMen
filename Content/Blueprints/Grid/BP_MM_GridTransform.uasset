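; BP_MM_GridTransform is a placeable actor that marks a grid's transform, with a preview mesh for visualizing the grid in the editor.
; The construction script scales the mesh from PreviewGridSize, mapping width to Y and height to Z with X as forward.
; It raises the mesh by half the grid's height, assuming 100 units per cell.
; BeginPlay destroys the preview mesh, since it is only needed at editor time.
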(event `self.ReceiveBeginPlay`
  ;[1 1 1] Only needed at editor time
  (bind _previewgridmesh (`self.PreviewGridMesh`)
    (:`then`
      (`ActorComponent.K2_DestroyComponent` _previewgridmesh))
    (:`else`)))

(fn `UserConstructionScript`
  (bind (_x _y) (`KismetMathLibrary.BreakVector2D` (`self.PreviewGridSize`)))
  ;[1 1 1] X is forward, so horizontal axis is Y, and vertical axis is Z
  (`SceneComponent.SetWorldScale3D` (`self.PreviewGridMesh`) (`KismetMathLibrary.MakeVector` 1.0 _x _y))
  ;[1 1 1] Height Offset
  (`SceneComponent.K2_SetRelativeLocation` (`self.PreviewGridMesh`) (`KismetMathLibrary.MakeVector` 0.0 0.0 (/ (* (`.Y` (`KismetMathLibrary.BreakVector2D` (`self.PreviewGridSize`))) 100.0) 2.0)) false false))